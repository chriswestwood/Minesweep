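; BP_Tile is a grid tile actor that displays the revealed face of a Minesweeper-style cell.
; Its ShowTile event takes a flag M and a number C, then swaps the TileSprite image.
; A true M shows the bomb sprite; otherwise a switch on C picks the matching numbered sprite, with zero or any unmatched value showing a blank tile.
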(event `self.ShowTile`
  (params (m :type Boolean) (c :type Integer))
  (bind _tilesprite (`self.TileSprite`))
  (if m
    (`PaperSpriteComponent.SetSprite` _tilesprite "/Game/Assets/tileset_tile_bomb.tileset_tile_bomb")
    (else
      (switch `int` c
        (:`Default`
          (`PaperSpriteComponent.SetSprite` _tilesprite "/Game/Assets/tileset_tile_blank.tileset_tile_blank" :!label _label))
        (:`0`
          (goto _label))
        (:`1`
          (`PaperSpriteComponent.SetSprite` _tilesprite "/Game/Assets/tileset_tile_1.tileset_tile_1"))
        (:`2`
          (`PaperSpriteComponent.SetSprite` _tilesprite "/Game/Assets/tileset_tile_2.tileset_tile_2"))
        (:`3`
          (`PaperSpriteComponent.SetSprite` _tilesprite "/Game/Assets/tileset_tile_3.tileset_tile_3"))
        (:`4`
          (`PaperSpriteComponent.SetSprite` _tilesprite "/Game/Assets/tileset_tile_4.tileset_tile_4"))
        (:`5`
          (`PaperSpriteComponent.SetSprite` _tilesprite "/Game/Assets/tileset_tile_5.tileset_tile_5"))
        (:`6`
          (`PaperSpriteComponent.SetSprite` _tilesprite "/Game/Assets/tileset_tile_6.tileset_tile_6"))
        (:`7`
          (`PaperSpriteComponent.SetSprite` _tilesprite "/Game/Assets/tileset_tile_7.tileset_tile_7"))
        (:`8`
          (`PaperSpriteComponent.SetSprite` _tilesprite "/Game/Assets/tileset_tile_8.tileset_tile_8"))))))

(fn `UserConstructionScript`)